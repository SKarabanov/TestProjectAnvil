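; AI controller for BP_AI_Char pawns that drives them with the BT_AI_Base behavior tree.
; On possession it caches the character, and on BeginPlay it starts the tree, stores the first player character as the TargetCharacter blackboard key and sets an initial state.
; SetNewState writes the state to the character and mirrors it into the AI_State blackboard key.
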(event EventBeginPlay
  (AI|RunBehaviorTree "/Game/TestWork/AI/BT_AI_Base.BT_AI_Base")
  (bind _blackboard (Variables|Default|GetBlackboard)
    (:then
      (AI|Components|Blackboard|SetValueasObject _blackboard (Utilities|Name|MakeLiteralName "TargetCharacter") (Game|GetPlayerCharacter 0))
      (CallFunction|SetNewState "NewEnumerator0"))
    (:else)))

(event EventPossess
  (params (PossessedPawn :type Pawn%20Object%20Reference))
  (bind _asbp_ai_char (Utilities|Casting|CastToBP_AI_Char PossessedPawn))
  (Variables|Default|SetChar _asbp_ai_char))

(fn ConstructionScript)

(fn SetNewState
  (params (State :type E_AI_State%20Enum :default "NewEnumerator0"))
  (bind _output_get (Variables|/Game/TestWork/BP_AI_Char.BP_AI_Char_C|SetState (Variables|Default|GetChar) State))
  (bind _blackboard (Variables|Default|GetBlackboard)
    (:then
      (AI|Components|Blackboard|SetValueasEnum _blackboard (Utilities|Name|MakeLiteralName "AI_State") _output_get))
    (:else)))