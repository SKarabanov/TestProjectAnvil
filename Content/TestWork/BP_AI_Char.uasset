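; BP_AI_Char is an AI character that turns to face the first player character while in State 2.
; BeginPlay caches that player as Target, and Tick calls RotateCharacterToTarget only for that state.
; The function fetches the player again rather than reading Target, then interpolates yaw toward it at constant speed, using the movement component's yaw RotationRate.
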(event EventTick
  (params (DeltaSeconds :type Float%20%28single-precision%29))
  ;[1 1 1] Rotate char to Target every Tick
  (switch Utilities|FlowControl|Switch|SwitchonE_AI_State (Variables|Default|GetState)
    (:NewEnumerator1
      (CallFunction|RotateCharactertoTarget))))

(event EventBeginPlay
  (bind _returnvalue (Game|GetPlayerCharacter 0))
  (Utilities|IsValid _returnvalue
    (:Is%20Valid
      (Variables|Default|SetTarget _returnvalue))))

(fn ConstructionScript)

(fn RotateCharactertoTarget
  (Transformation|SetActorRotation (Class|KismetMathLibrary|RInterptoConstant (Math|Rotator|MakeRotator 0.0 0.0 (.yaw (Transformation|GetActorRotation))) (Math|Rotator|MakeRotator 0.0 0.0 (.yaw (Math|Rotator|FindLookatRotation (Transformation|GetActorLocation) (Transformation|GetActorLocation (Game|GetPlayerCharacter 0))))) (Utilities|Time|GetWorldDeltaSeconds) (.yaw (Variables|/Script/Engine.CharacterMovementComponent|GetRotationRate (Variables|Character|GetCharacterMovement))))))